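; Networked projectile actor that flies along its Rotation variable at a set Speed and damages what its capsule overlaps.
; BeginPlay sets the movement component's velocity, and the server destroys the actor after a short lifetime.
; On overlap it applies damage without an authority check, then branches on collision object type: pawns get a bullet-impact emitter, other handled types spawn an explosion effect actor.
; Both branches end in server-only destruction.
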(event OnComponentBeginOverlap(Capsule)
  (params (OverlappedComponent :type Primitive%20Component%20Object%20Reference) (OtherActor :type Actor%20Object%20Reference) (OtherComp :type Primitive%20Component%20Object%20Reference) (OtherBodyIndex :type Integer) (bFromSweep :type Boolean) (SweepResult :type Hit%20Result%20Structure%20%28by%20ref%29))
  (Game|Damage|ApplyDamage OtherActor (Variables|Default|GetDamage) 0 0)
  (switch Utilities|FlowControl|Switch|SwitchonECollisionChannel (Collision|GetCollisionObjectType OtherComp)
    (:ECC_WorldStatic
      (Game|SpawnActorfromClass "/Game/StarterContent/Blueprints/Blueprint_Effect_Explosion.Blueprint_Effect_Explosion_C" (Math|Transform|MakeTransform (Transformation|GetActorLocation) (Transformation|GetActorRotation)) "Undefined" 0 0 :!label _label))
    (:ECC_WorldDynamic
      (goto _label))
    (:ECC_Pawn
      (Effects|SpawnEmitteratLocation "/Game/FX/P_body_bullet_impact.P_body_bullet_impact" (Transformation|GetActorLocation) (Transformation|GetActorRotation)))
    (:ECC_PhysicsBody
      (goto _label))
    (:ECC_Vehicle
      (goto _label))
    (:ECC_Destructible
      (goto _label)))
  (Networking|SwitchHasAuthority
    (:Authority
      (Actor|DestroyActor))))

(event EventBeginPlay
  (Variables|/Script/Engine.MovementComponent|SetVelocity (Variables|Default|GetProjectileMovement) (* (Math|Vector|GetForwardVector (Variables|Default|GetRotation)) (Variables|Default|GetSpeed)))
  (Networking|SwitchHasAuthority
    (:Authority
      (Utilities|FlowControl|Delay 5.0)
      (Actor|DestroyActor))))

(fn ConstructionScript)