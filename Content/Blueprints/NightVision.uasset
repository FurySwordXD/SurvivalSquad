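; Battery-powered night vision Blueprint that toggles three spotlights and manages their charge.
; A looping timer drains charge while lit and bright, then a one-shot timeline fades the lights at zero.
; Reload spends a battery to ramp intensity and charge through a shared timeline, which also plays on first switch-on.
; Switch-off disables the NightVision post-process, but the node enabling it is disconnected.
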(event Custom|ToggleNightVision
  (if (Variables|Default|GetOn?)
    (Rendering|SetVisibility (Variables|Default|GetSpotLight) false false)
    (Variables|/Script/Engine.PostProcessComponent|SetbEnabled (Variables|Default|GetNightVision) false)
    (Variables|Default|SetOn? false)
    (else
      (Rendering|SetVisibility (Variables|Default|GetSpotLight2) true false)
      (Variables|Default|SetOn? true)
      (Utilities|FlowControl|DoOnce false
        (:Completed
          (CallFunction|IntensityGain false))))))

(event Custom|IntensityDrop
  ;[1 1 1] NightVision
  (if (<= (Variables|Default|GetCharge) 0)
    (Utilities|FlowControl|DoOnce false
      (:Completed
        (bind _intensitydrop (Timeline|Timeline_0 PlayFromStart)
          (:Update
            (Rendering|Components|Light|SetIntensity (Variables|Default|GetSpotLight) _intensitydrop)))))))

(event Custom|IntensityGain
  (params (IncreaseCharge? :type Boolean))
  ;[1 1 1] NightVision
  (bind _alpha (Timeline|Timeline_1 PlayFromStart)
    (:Update
      (Rendering|Components|Light|SetIntensity (Variables|Default|GetSpotLight) (Math|Float|Lerp 0.0 2.333e+04 _alpha))
      (Rendering|Components|Light|SetIntensity (Variables|Default|GetSpotLight1) (Math|Float|Lerp 0.0 8.318e+04 _alpha))
      (Rendering|Components|Light|SetIntensity (Variables|Default|GetSpotLight2) (Math|Float|Lerp 0.0 4.527e+04 _alpha))
      (if IncreaseCharge?
        (Variables|Default|SetCharge (Math|Integer|Clamp(Integer) (Math|Float|Truncate (Math|Float|Lerp 0.0 6e+02 _alpha)) 0 (Variables|Default|GetMaxCharge)))))))

(event Custom|Reload
  (bind _batteries (Variables|Default|GetBatteries))
  ;[1 1 1] NightVision
  (if (and (> _batteries 0) (< (Variables|Default|GetCharge) (Variables|Default|GetMaxCharge)))
    (CallFunction|IntensityGain true)
    (Math|Integer|DecrementInt _batteries)))

(event EventBeginPlay
  (Utilities|Time|SetTimerbyFunctionName 0 "ChargeDrop" (Variables|Default|GetTimer) true))

(fn ConstructionScript)

(fn ChargeDrop
  (if (and (Variables|Default|GetOn?) (>= (Variables|/Script/Engine.LightComponentBase|GetIntensity (Variables|Default|GetSpotLight)) 4e+03))
    (Math|Integer|DecrementInt (Variables|Default|GetCharge)
      (:%20%20
        _)))
  (CallFunction|IntensityDrop))