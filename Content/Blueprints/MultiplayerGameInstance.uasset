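; A multiplayer Game Instance Blueprint that wraps online session hosting, joining and teardown for the first local player controller.
; Host creates a session with a given player limit and LAN flag, then opens the named level as a listen server.
; Join connects to the indexed entry in Sessions, which this graph never fills, and Destroy ends the session.
; Successful hosting or joining hides the mouse cursor and switches input to game-only.
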(event Custom|Host
  (params (LevelName :type String) (MaxPlayers :type Integer) (bUseLAN :type Boolean))
  (bind _returnvalue (Game|GetPlayerController 0))
  (|Session (Game|GetPlayerController 0) MaxPlayers bUseLAN
    (:OnSuccess
      (Game|OpenLevel(byName) (Utilities|String|StringToName LevelName) true "listen")
      (Variables|/Script/Engine.PlayerController|SetbShowMouseCursor _returnvalue false)
      (Input|SetInputModeGameOnly _returnvalue))))

(event Custom|Destroy
  (|DestroySession (Game|GetPlayerController 0)))

(event Custom|Join
  (bind _returnvalue (Game|GetPlayerController 0))
  (bind _sessionindex (Variables|Default|GetSessionIndex))
  (if (>= _sessionindex 0)
    (|JoinSession (Game|GetPlayerController 0) (Utilities|Array|Get(acopy) (Variables|Default|GetSessions) _sessionindex)
      (:OnSuccess
        (Variables|/Script/Engine.PlayerController|SetbShowMouseCursor _returnvalue false)
        (Input|SetInputModeGameOnly _returnvalue)))))