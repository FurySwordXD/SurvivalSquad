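; DoorBP is an interactable door that swings its static mesh open or closed on each Interact call.
; Opening first compares player and door forward vectors to pick a swing sign, then plays a timeline whose value times that sign sets the mesh yaw.
; Closing reverses the timeline, keeping the sign.
; Interaction is blocked during movement, and Open follows the timeline direction on finish; collision toggles are present but never run.
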(event EventInteract
  (params (Player :type Third%20Person%20Character%20Object%20Reference))
  (if (Variables|Default|GetCanInteract?)
    (if (Variables|Default|GetOpen?)
      (bind (_direction _newtrack_0) (Timeline|Timeline_0 Reverse)
        (:Update
          (Variables|Default|SetCanInteract? false)
          (Transformation|SetRelativeRotation (Variables|Default|GetStaticMesh) (Math|Rotator|MakeRotator 0.0 0.0 (* _newtrack_0 (Variables|Default|Get1/-1))) false false))
        (:Finished
          (Variables|Default|SetCanInteract? true)
          (if (Utilities|Enum|Equal(Enum) _direction "Forward")
            (Variables|Default|SetOpen? true)
            (else
              (Variables|Default|SetOpen? false)))))
      (else
        (Variables|Default|Set1/-1 (select (> (Class|KismetMathLibrary|DegAcos (Math|Vector|DotProduct (Transformation|GetActorForwardVector Player) (Transformation|GetActorForwardVector))) 9e+01) -1.0 1.0))
        (Timeline|Timeline_0 Play)))))

(fn ConstructionScript
  (|CallParentFunction))