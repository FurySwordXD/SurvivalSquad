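; World pickup actor that holds an item class and amount for transfer into a player's inventory.
; Interact calls PickUp, which adds the item through the target's InventoryComponent.
; On success it subtracts any returned Rest from Amount, or destroys itself when no Rest remains.
; EnterBox lists the pickup in the player's pickup widget, passing the item class defaults, amount and itself.
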(event Custom|PickUp
  (params (Target :type Third%20Person%20Character%20Object%20Reference))
  (bind (_success_ _rest) (Default|AddItem (Variables|/Game/ThirdPersonBP/Blueprints/ThirdPersonCharacter.ThirdPersonCharacter_C|GetInventoryComponent Target) (Variables|Default|GetItemClass) (Variables|Default|GetAmount)))
  (if _success_
    (if (> _rest 0)
      (Variables|Default|SetAmount (- (Variables|Default|GetAmount) _rest))
      (else
        (Actor|DestroyActor)))))

(event EventEnterBox
  (params (Player :type Third%20Person%20Character%20Object%20Reference))
  (Default|AddPickUp (Variables|/Game/InventorySystem/Widgets/MainWidget.MainWidget_C|GetPickUpWidget_104 (Variables|/Game/InventorySystem/InventoryComponent.InventoryComponent_C|GetMainWidget (Variables|/Game/ThirdPersonBP/Blueprints/ThirdPersonCharacter.ThirdPersonCharacter_C|GetInventoryComponent Player))) (Utilities|GetClassDefaults (Variables|Default|GetItemClass)) (Variables|Default|GetAmount) self))

(event EventInteract
  (params (Player :type Third%20Person%20Character%20Object%20Reference))
  (CallFunction|PickUp Player))

(fn ConstructionScript
  (|CallParentFunction))